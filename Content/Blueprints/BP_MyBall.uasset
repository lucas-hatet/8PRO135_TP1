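; BP_MyBall is a ball actor that removes itself when it touches an asteroid or travels too far along world X.
; Tick checks the root component's world position and destroys the ball once X reaches a fixed limit.
; The Sphere's begin-overlap event destroys it only when the other actor's class is exactly BP_MyAsteroid.
; The graph contains no movement logic and does nothing to the asteroid itself.
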(event OnComponentBeginOverlap(Sphere)
  (params (OverlappedComponent :type Primitive%20Component%20Object%20Reference) (OtherActor :type Actor%20Object%20Reference) (OtherComp :type Primitive%20Component%20Object%20Reference) (OtherBodyIndex :type Integer) (bFromSweep :type Boolean) (SweepResult :type Hit%20Result%20Structure%20%28by%20ref%29))
  (if (== (Utilities|GetClass OtherActor) "/Game/Blueprints/BP_MyAsteroid.BP_MyAsteroid_C")
    (Actor|DestroyActor)))

(event EventBeginPlay)

(event Collision|EventActorBeginOverlap
  (params (OtherActor :type Actor%20Object%20Reference)))

(event EventTick
  (params (DeltaSeconds :type Float%20%28single-precision%29))
  (if (>= (.X (Math|Vector|BreakVector (Transformation|GetWorldLocation (Variables|Default|GetDefaultSceneRoot)))) 3.5e+03)
    (Actor|DestroyActor)))

(fn ConstructionScript)