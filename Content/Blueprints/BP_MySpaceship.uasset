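; BP_MySpaceship is the player's spaceship, handling asteroid hits and XP pickups through its static mesh's overlap event.
; Lives and score live in BPI_GameInstance, with lives reset on BeginPlay.
; Asteroids cost a life and XP adds score, both destroyed on contact, except the fatal asteroid: the ship hides and the Menu level opens.
; Tick pins the spring arm to a fixed world rotation.
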(event OnComponentBeginOverlap(StaticMesh)
  (params (OverlappedComponent :type Primitive%20Component%20Object%20Reference) (OtherActor :type Actor%20Object%20Reference) (OtherComp :type Primitive%20Component%20Object%20Reference) (OtherBodyIndex :type Integer) (bFromSweep :type Boolean) (SweepResult :type Hit%20Result%20Structure%20%28by%20ref%29))
  (bind _returnvalue (Utilities|GetClass OtherActor))
  (bind _asbpi_game_instance (Utilities|Casting|CastToBPI_GameInstance (Game|GetGameInstance)))
  (if (== _returnvalue "/Game/Blueprints/BP_MyAsteroid.BP_MyAsteroid_C")
    (bind _result (Math|Integer|DecrementInt (Variables|/Game/Blueprints/BPI_GameInstance.BPI_GameInstance_C|GetVie _asbpi_game_instance))
      (:%20%20
        (bind _output_get (Variables|/Game/Blueprints/BPI_GameInstance.BPI_GameInstance_C|SetVie _asbpi_game_instance _result))
        (if (<= _output_get 0)
          (Rendering|SetActorHiddenInGame (Components|GetOwner (Variables|Default|GetStaticMesh)) true)
          (Game|OpenLevel(byObjectReference) "/Game/Maps/Menu.Menu")
          (else
            (Actor|DestroyActor OtherActor :!label _label)))))
    (elif (== _returnvalue "/Game/Blueprints/BP_MyXp.BP_MyXp_C")
      (Variables|/Game/Blueprints/BPI_GameInstance.BPI_GameInstance_C|SetScore _asbpi_game_instance (+ (Variables|/Game/Blueprints/BPI_GameInstance.BPI_GameInstance_C|GetScore _asbpi_game_instance) 5))
      (goto _label))))

(event EventBeginPlay
  (bind _asbpi_game_instance (Utilities|Casting|CastToBPI_GameInstance (Game|GetGameInstance)))
  (Variables|/Game/Blueprints/BPI_GameInstance.BPI_GameInstance_C|SetVie _asbpi_game_instance 3))

(event Collision|EventActorBeginOverlap
  (params (OtherActor :type Actor%20Object%20Reference)))

(event EventTick
  (params (DeltaSeconds :type Float%20%28single-precision%29))
  (Transformation|SetWorldRotation (Variables|Default|GetSpringArm) "-50.000000,0.000000,0.000000" false false))

(fn ConstructionScript)