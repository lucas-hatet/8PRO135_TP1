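; Asteroid actor that drifts along negative X, speeding up with the game instance's score, and destroys itself past a rear limit.
; On BeginPlay it randomizes its scale per axis and shows one of three meshes.
; Sphere overlaps with BP_MyBall give rising destruction odds, guaranteed by the fifth hit, and spawn BP_MyXp on destruction.
; Touching BP_MySpaceship destroys it without spawning XP.
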(event OnComponentBeginOverlap(Sphere)
  (params (OverlappedComponent :type Primitive%20Component%20Object%20Reference) (OtherActor :type Actor%20Object%20Reference) (OtherComp :type Primitive%20Component%20Object%20Reference) (OtherBodyIndex :type Integer) (bFromSweep :type Boolean) (SweepResult :type Hit%20Result%20Structure%20%28by%20ref%29))
  (bind _returnvalue (Utilities|GetClass OtherActor))
  (if (== _returnvalue "/Game/Blueprints/BP_MyBall.BP_MyBall_C")
    (if (== (Class|KismetMathLibrary|RandomInteger64 (- 5 (Variables|Default|GetNbHit))) 0)
      (Game|SpawnActorfromClass "/Game/Blueprints/BP_MyXp.BP_MyXp_C" (Math|Transform|MakeTransform (Transformation|GetWorldLocation OverlappedComponent)) "Undefined" "MultiplyWithRoot" 0 0)
      (Actor|DestroyActor :!label _label)
      (else
        (bind _result (Math|Integer|IncrementInt (Math|Conversions|ToInteger(Byte) (Variables|Default|GetNbHit)))
          (:%20%20
            (Variables|Default|SetNbHit (Class|KismetMathLibrary|ToInt64(Integer) _result))))))
    (elif (== _returnvalue "/Game/Blueprints/BP_MySpaceship.BP_MySpaceship_C")
      (goto _label))))

(event EventBeginPlay
  (bind _returnvalue (Class|KismetMathLibrary|RandomInteger64inRange 1 6))
  (bind _asteroid1 (Variables|Default|GetAsteroid1))
  (bind _returnvalue_2 (Math|Conversions|ToFloat(Integer) _returnvalue))
  (Variables|Default|SetNbHit 0)
  (Transformation|SetActorScale3D (Math|Vector|MakeVector _returnvalue_2 _returnvalue_2 _returnvalue_2))
  (Rendering|SetVisibility _asteroid1 false false)
  (switch int (Math|Random|RandomIntegerinRange 0 2)
    (:Default
      (Rendering|SetVisibility _asteroid1 true false :!label _label))
    (:0
      (goto _label))
    (:1
      (Rendering|SetVisibility (Variables|Default|GetAsteroid2) true false))
    (:2
      (Rendering|SetVisibility (Variables|Default|GetAsteroid3) true false))))

(event Collision|EventActorBeginOverlap
  (params (OtherActor :type Actor%20Object%20Reference)))

(event EventTick
  (params (DeltaSeconds :type Float%20%28single-precision%29))
  (bind _asbpi_game_instance (Utilities|Casting|CastToBPI_GameInstance (Game|GetGameInstance)))
  (Transformation|AddActorWorldOffset (Math|Vector|MakeVector (- -5.0 (/ (Math|Conversions|ToFloat(Integer) (Variables|/Game/Blueprints/BPI_GameInstance.BPI_GameInstance_C|GetScore _asbpi_game_instance)) 4e+01)) 0.0 0.0))
  (if (<= (.X (Math|Vector|BreakVector (Transformation|GetWorldLocation (Variables|Default|GetSphere)))) -1e+03)
    (Actor|DestroyActor)))

(fn ConstructionScript)